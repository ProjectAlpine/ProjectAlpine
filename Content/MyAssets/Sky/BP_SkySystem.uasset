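; Sky system Blueprint that animates the sky by continuously rotating itself and its SunLight and MoonLight actors.
; Each Tick adds the same fixed world-rotation step to all three, without delta-time scaling, so speed depends on frame rate.
; A 24-hour GameTime clock and a time-to-rotation calculation are present but disconnected, so time of day does not drive the motion.
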(event `self.ReceiveTick`
  (params (DeltaSeconds :type "Float (single-precision)"))
  (`|ExecutionSequence`
    (:`then_0`
      (`self.K2_AddActorWorldRotation` (struct :`Pitch` 0.1)))
    (:`then_1`
      (`self.K2_AddActorWorldRotation` (`self.SunLight`) (struct :`Pitch` 0.1) false false))
    (:`then_2`
      (`self.K2_AddActorWorldRotation` (`self.MoonLight`) (struct :`Pitch` 0.1) false false))))

(fn `UserConstructionScript`)